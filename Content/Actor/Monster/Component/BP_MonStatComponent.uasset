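; Monster stat component that holds a monster's data and current HP and broadcasts changes through event dispatchers.
; SetMonState loads a DT_Monster row by name, starts HP at that row's value and broadcasts the stats.
; AddDamage adds a signed value to HP, broadcasts the update and fires Death at zero or below.
; IsDeath always returns false, so its guard never blocks further damage or repeated Death calls.
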(fn `AddDamage`
  (params (Damage :type "Float (double-precision)"))
  (bind (_curmonstat_mondata _curmonstat_curhp) (break `/Game/Actor/Monster/Data/ST_CurMonster` (`self.CurMonStat`)))
  (bind _curmonstat (`self.CurMonStat`))
  (if (not (`self.IsDeath`))
    (bind _structout (setmembers `/Game/Actor/Monster/Data/ST_CurMonster` :`StructRef` (`self.CurMonStat`) :`CurHp` (+ _curmonstat_curhp Damage)))
    (`self.EventDispatcher_UpdateHp` (`.CurHp_5_5A39D35F409DD603B988B78D45475DE1` (break `/Game/Actor/Monster/Data/ST_CurMonster` _curmonstat)) (`.Hp_9_5287BF4A466EF8FCA3D19F902E4AD213` (break `/Game/Actor/Monster/Data/ST_Monster` (break `/Game/Actor/Monster/Data/ST_CurMonster` _curmonstat))))
    (if (<= (`.CurHp_5_5A39D35F409DD603B988B78D45475DE1` (break `/Game/Actor/Monster/Data/ST_CurMonster` _structout)) 0.0)
      (`self.EventDispatcher_Death` (`self.CurMonStat`)))))

(fn `IsDeath`
  (returns (IsDeath :type Boolean))
  (return false))

(fn `SetMonState`
  (params (RowName :type Name))
  (bind _returnvalue (`|GetDataTableRow` "/Game/Actor/Monster/Data/DT_Monster.DT_Monster" RowName)
    (:`then`
      (bind _output_get (set `self.CurMonStat` (make `/Game/Actor/Monster/Data/ST_CurMonster` _returnvalue (`.Hp_9_5287BF4A466EF8FCA3D19F902E4AD213` (break `/Game/Actor/Monster/Data/ST_Monster` _returnvalue)))))
      (`self.EventDispatcher_MonStat` _output_get))))