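; Player skill actor for a ball that orbits its Character and deals area damage, destroying itself after ten seconds.
; Each Tick, RotateFunc advances an angle by RotationSpeed and uses sine and cosine to place the actor on a horizontal circle of clamped radius around the Character.
; DoDamage accumulates delta time to apply periodic radial damage at the Rotation component, ignoring the Character and crediting its controller.
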(event `self.ReceiveBeginPlay`
  (`KismetSystemLibrary.Delay` 10.0)
  (`self.K2_DestroyActor`))

(event `self.ReceiveTick`
  (params (DeltaSeconds :type "Float (single-precision)"))
  (`|ExecutionSequence`
    (:`then_0`
      (`self.RotateFunc` DeltaSeconds))
    (:`then_1`
      (`self.DoDamage` DeltaSeconds))))

(fn `DoDamage`
  (params (DeltaSeconds :type "Float (double-precision)"))
  (bind _character (`self.Character`))
  (bind _output_get (set `self.DamageDelay` (+ DeltaSeconds (`self.DamageDelay`))))
  (if (> _output_get 0.1)
    (set `self.DamageDelay` 0.0)
    (`GameplayStatics.ApplyRadialDamage` 10.0 (`SceneComponent.K2_GetComponentLocation` (`self.Rotation`)) 100.0 null (`|MakeArray` _character :!type "Actor Object Reference") self (`Pawn.GetController` _character))))

(fn `RotateFunc`
  (params (DeltaSeconds :type "Float (double-precision)"))
  (locals (Center :type "Vector Structure" :default (0.0 0.0 0.0)) (RotationSpeed :type "Float (double-precision)" :default 50.0) (AngleRadians :type "Float (double-precision)") (OrbitRadius :type "Float (double-precision)" :default 250.0) (Offset :type "Vector Structure"))
  (bind _angleradians (`local.AngleRadians`))
  (bind _orbitradius (`local.OrbitRadius`))
  (bind _output_get (set `self.CurrentAngle` (+ (* DeltaSeconds (`local.RotationSpeed`)) (`self.CurrentAngle`))))
  (set `local.AngleRadians` (`KismetMathLibrary.DegreesToRadians` _output_get))
  (set `local.OrbitRadius` (`KismetMathLibrary.FClamp` (`local.OrbitRadius`) 200.0 300.0))
  (set `local.Center` (`self.K2_GetActorLocation` (`self.Character`)))
  (bind _output_get_2 (set `local.Offset` (`KismetMathLibrary.MakeVector` (* (`KismetMathLibrary.Cos` _angleradians) _orbitradius) (* _orbitradius (`KismetMathLibrary.Sin` _angleradians)))))
  (`self.K2_SetActorLocation` (+ _output_get_2 (`local.Center`))))

(fn `UserConstructionScript`
  (`parent.UserConstructionScript`))