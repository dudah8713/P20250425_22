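; BP_Fireball is a player skill projectile that damages what is around it as it flies and destroys itself after five seconds.
; Tick moves the Fireball component along the actor's forward vector at Speed without sweeping, so it does not stop on collisions.
; Tick also feeds DoDamage, which accumulates delta time to periodically apply radial damage at the fireball's location, ignoring Character and crediting its controller.
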(event `self.ReceiveBeginPlay`
  (`KismetSystemLibrary.Delay` 5.0)
  (`self.K2_DestroyActor`))

(event `self.ReceiveTick`
  (params (DeltaSeconds :type "Float (single-precision)"))
  (`|ExecutionSequence`
    (:`then_0`
      (`SceneComponent.K2_AddWorldOffset` (`self.Fireball`) (* (`self.GetActorForwardVector`) (* DeltaSeconds (`self.Speed`))) false false))
    (:`then_1`
      (`self.DoDamage` DeltaSeconds))))

(fn `DoDamage`
  (params (DeltaSeconds :type "Float (double-precision)"))
  (bind _character (`self.Character`))
  (bind _output_get (set `self.DamageDelay` (+ DeltaSeconds (`self.DamageDelay`))))
  (if (> _output_get 0.1)
    (set `self.DamageDelay` 0.0)
    (`GameplayStatics.ApplyRadialDamage` 15.0 (`SceneComponent.K2_GetComponentLocation` (`self.Fireball`)) 100.0 null (`|MakeArray` _character :!type "Actor Object Reference") self (`Pawn.GetController` _character))))

(fn `UserConstructionScript`)