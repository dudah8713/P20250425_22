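; BP_Slash is a short-lived player skill actor that plays a slash effect and deals area damage.
; On BeginPlay it snaps a component onto the owning Character's mesh and applies radial damage once at its own location, ignoring that Character and crediting its controller.
; The Slash effect's system-finished event drives cleanup, with EventFinishAttack destroying the actor, so its lifetime follows the effect.
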(event `self.ReceiveBeginPlay`
  (bind _character (`self.Character`))
  (add `NiagaraComponent.OnSystemFinished` (`self.Slash`) (`|CreateDelegate` :!event `EventFinishAttack`))
  (`self.K2_AttachToComponent` (`Character.Mesh` (`self.Character`)) "None" "SnapToTarget" "SnapToTarget" "KeepWorld")
  (`GameplayStatics.ApplyRadialDamage` 30.0 (`self.K2_GetActorLocation`) 0.0 null (`|MakeArray` _character :!type "Actor Object Reference") self (`Pawn.GetController` _character)))

(fn `EventFinishAttack`
  (params (PSystem :type "NiagaraComponent Object Reference"))
  (`self.K2_DestroyActor`))

(fn `UserConstructionScript`
  (`parent.UserConstructionScript`))