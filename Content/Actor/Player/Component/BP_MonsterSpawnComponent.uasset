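; Player component that periodically spawns random monsters on a ring around the player.
; A looping timer started at BeginPlay picks a random angle at CircleRadius from the first player controller's location.
; A short downward line trace accepts the point only if it hits static or dynamic world objects.
; A random DT_Monster row then supplies the class for SpawnAIFromClass, and its row name is passed to BP_MonsterBase's SetMonState.
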(event `self.ReceiveBeginPlay`
  (`KismetSystemLibrary.K2_SetTimer` null "SpawnMonster" 1.0 true))

(fn `GetRandomCircleLocation`
  (returns (SpawnLocation :type "Vector Structure"))
  (locals (RandLocation :type "Vector Structure") (RandRowName :type Name) (CircleRadius :type "Float (double-precision)" :default 1500.0) (RandAngle :type "Float (double-precision)") (PlayerLocation :type "Vector Structure"))
  (bind _circleradius (`local.CircleRadius`))
  (bind _output_get (set `local.RandAngle` (`KismetMathLibrary.RandomFloatInRange` 0.0 360.0)))
  (bind _output_get_2 (set `local.PlayerLocation` (`Actor.K2_GetActorLocation` (`GameplayStatics.GetPlayerController` 0))))
  (bind _returnvalue (`KismetMathLibrary.DegreesToRadians` _output_get))
  (return (+ _output_get_2 (`KismetMathLibrary.MakeVector` (* (`KismetMathLibrary.Cos` _returnvalue) _circleradius) (* _circleradius (`KismetMathLibrary.Sin` _returnvalue))))))

(fn `IsCanSpawnLocation`
  (params (SpawnLocation :type "Vector Structure"))
  (returns (CanSpawn :type Boolean))
  (bind (_outhit _returnvalue) (`KismetSystemLibrary.LineTraceSingleForObjects` SpawnLocation (- SpawnLocation (0.0 0.0 100.0)) (`|MakeArray` "ObjectTypeQuery1" "ObjectTypeQuery2" :!type "EObjectTypeQuery Enum")))
  (return _returnvalue))

(fn `SpawnMonster`
  (locals (RandSpawnLocation :type "Vector Structure") (RandRowName :type Name))
  (bind _output_get (set `local.RandSpawnLocation` (`self.GetRandomCircleLocation`)))
  (if (`self.IsCanSpawnLocation` _output_get)
    (bind _outrownames (`DataTableFunctionLibrary.GetDataTableRowNames` "/Game/Actor/Monster/Data/DT_Monster.DT_Monster"))
    (bind _output_get_2 (set `local.RandRowName` (`KismetArrayLibrary.Array_Random` _outrownames)))
    (bind _returnvalue (`|GetDataTableRow` "/Game/Actor/Monster/Data/DT_Monster.DT_Monster" _output_get_2)
      (:`then`
        (bind _returnvalue_2 (`AIBlueprintHelperLibrary.SpawnAIFromClass` (`.MonsterClass_6_E6AE458E4325C8D61CF1D0A7E3871E3A` (break `/Game/Actor/Monster/Data/ST_Monster` _returnvalue)) null (`local.RandSpawnLocation`) (struct) false null))
        (bind _asbp_monster_base (cast `/Game/Actor/Monster/BP_MonsterBase` _returnvalue_2))
        (`/Game/Actor/Monster/BP_MonsterBase.SetMonState` _asbp_monster_base (`local.RandRowName`))))))