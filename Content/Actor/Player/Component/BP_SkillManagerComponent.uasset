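; Player skill manager component that automatically casts each held skill whenever its cooldown elapses.
; AddSkills fills the Skills array from every DT_Skill row, starting each timer at its full cooldown so the first cast is almost immediate.
; Tick advances every timer, and on expiry spawns that skill's SkillBase actor at the owner's transform, passes in the owning Character, and resets the timer.
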(event `self.ReceiveTick`
  (params (DeltaSeconds :type "Float (single-precision)"))
  (`self.UpdateSkill` DeltaSeconds))

(fn `AddSkills`
  (bind _outrownames (`DataTableFunctionLibrary.GetDataTableRowNames` "/Game/Actor/Player/Data/DT_Skill.DT_Skill"))
  (for _array_element _outrownames
    (bind _returnvalue (`|GetDataTableRow` "/Game/Actor/Player/Data/DT_Skill.DT_Skill" _array_element)
      (:`then`
        (`KismetArrayLibrary.Array_Add` (`self.Skills`) (make `/Game/Actor/Player/Data/ST_CurSkill` _returnvalue (`.CoolTime_9_9292EDE14558EF3934B33B8CBB36FD4D` (break `/Game/Actor/Player/Data/ST_Skill` _returnvalue))))))))

(fn `DoUseSkill`
  (params (CurSkill :type "/Game/Actor/Player/Data/ST_CurSkill Structure"))
  (bind _returnvalue (`self.GetOwner`))
  (bind _ascharacter (cast `Character` _returnvalue))
  (`|SpawnActorFromClass` (`.SkillBase_7_C5F281CA4A7109207879C992DCB2256B` (break `/Game/Actor/Player/Data/ST_Skill` (`.SkillData_5_F3AA61CC4BF4638EFF2B33A72A8A465B` (break `/Game/Actor/Player/Data/ST_CurSkill` CurSkill)))) (`Actor.GetTransform` _returnvalue) "Undefined" "MultiplyWithRoot" null _ascharacter null))

(fn `UpdateSkill`
  (params (DeltaSeconds :type "Float (double-precision)"))
  (for (_ _array_index) (`self.Skills`)
    (`self.UpdateSkillCoolTime` (`local.DeltaSeconds`) (`|GetArrayItem` (`self.Skills`) _array_index))))

(fn `UpdateSkillCoolTime`
  (params (DeltaSeconds :type "Float (double-precision)") (CurSKill :type "/Game/Actor/Player/Data/ST_CurSkill Structure (by ref)"))
  (locals (NewLocalVar :type "/Game/Actor/Player/Data/ST_Skill Structure"))
  (bind _structout (setmembers `/Game/Actor/Player/Data/ST_CurSkill` :`StructRef` CurSKill :`CurCoolTime` (+ (`.CurCoolTime_6_2539EE8F44CC61EB70AABA9999720496` (break `/Game/Actor/Player/Data/ST_CurSkill` CurSKill)) (`local.DeltaSeconds`))))
  (bind (_skilldata _curcooltime) (break `/Game/Actor/Player/Data/ST_CurSkill` _structout))
  (if (> _curcooltime (`.CoolTime_9_9292EDE14558EF3934B33B8CBB36FD4D` (break `/Game/Actor/Player/Data/ST_Skill` _skilldata)))
    (`self.DoUseSkill` _structout)
    (setmembers `/Game/Actor/Player/Data/ST_CurSkill` :`StructRef` _structout :`CurCoolTime` 0.0)))